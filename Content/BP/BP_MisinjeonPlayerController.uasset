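; Player controller for Misinjeon that opens menus and runs NPC dialogue and monologues for the player character Seori.
; Input actions for chat, screen, inventory, map and charm each pause the game and focus a new UI stack widget in UI-only mode.
; Dialogue functions fetch lines and selectable answers from the game mode by chapter, level and index, feeding HUD widgets.
; Ending a conversation closes the widget and usually advances the level.
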(event `EnhancedInput|/Game/BP/ThirdPerson/ThirdPerson/Input/Actions/IA_UI_Chat`
  (params (ActionValue :type Boolean) (ElapsedSeconds :type "Float (double-precision)") (TriggeredSeconds :type "Float (double-precision)") (InputAction :type "InputAction Object Reference" :default "/Game/BP/ThirdPerson/ThirdPerson/Input/Actions/IA_UI_Chat.IA_UI_Chat"))
  ;[1 1 1] Chat
  (:`Triggered`
    (`GameplayStatics.SetGamePaused` true)
    (bind _returnvalue (`|CreateWidget` "/Game/BP/WBP/Play_WBP/Stack/WBP_ChatStack.WBP_ChatStack_C"))
    (`UserWidget.AddToViewport` _returnvalue 0)
    (`WidgetBlueprintLibrary.SetInputMode_UIOnlyEx` (`GameplayStatics.GetPlayerController` 0) _returnvalue)
    (`Widget.SetFocus` _returnvalue)))

(event `EnhancedInput|/Game/BP/ThirdPerson/ThirdPerson/Input/Actions/IA_UI_Screen`
  (params (ActionValue :type Boolean) (ElapsedSeconds :type "Float (double-precision)") (TriggeredSeconds :type "Float (double-precision)") (InputAction :type "InputAction Object Reference" :default "/Game/BP/ThirdPerson/ThirdPerson/Input/Actions/IA_UI_Screen.IA_UI_Screen"))
  ;[1 1 1] Pause
  (:`Triggered`
    (`GameplayStatics.SetGamePaused` true)
    (bind _returnvalue (`|CreateWidget` "/Game/BP/WBP/Play_WBP/Stack/WBP_PlayerStack.WBP_PlayerStack_C"))
    (`UserWidget.AddToViewport` _returnvalue 0)
    (`WidgetBlueprintLibrary.SetInputMode_UIOnlyEx` (`GameplayStatics.GetPlayerController` 0) _returnvalue)
    (`Widget.SetFocus` _returnvalue)))

(event `EnhancedInput|/Game/BP/ThirdPerson/ThirdPerson/Input/Actions/IA_UI_Inventory`
  (params (ActionValue :type Boolean) (ElapsedSeconds :type "Float (double-precision)") (TriggeredSeconds :type "Float (double-precision)") (InputAction :type "InputAction Object Reference" :default "/Game/BP/ThirdPerson/ThirdPerson/Input/Actions/IA_UI_Inventory.IA_UI_Inventory"))
  ;[1 1 1] Inventory
  (:`Triggered`
    (`GameplayStatics.SetGamePaused` true)
    (bind _returnvalue (`|CreateWidget` "/Game/BP/WBP/Play_WBP/Stack/WBP_Inventory_Stack.WBP_Inventory_Stack_C"))
    (`UserWidget.AddToViewport` _returnvalue 0)
    (`WidgetBlueprintLibrary.SetInputMode_UIOnlyEx` (`GameplayStatics.GetPlayerController` 0) _returnvalue)
    (`Widget.SetFocus` _returnvalue)))

(event `EnhancedInput|/Game/BP/ThirdPerson/ThirdPerson/Input/Actions/IA_UI_Map`
  (params (ActionValue :type Boolean) (ElapsedSeconds :type "Float (double-precision)") (TriggeredSeconds :type "Float (double-precision)") (InputAction :type "InputAction Object Reference" :default "/Game/BP/ThirdPerson/ThirdPerson/Input/Actions/IA_UI_Map.IA_UI_Map"))
  ;[1 1 1] Map
  (:`Triggered`
    (`GameplayStatics.SetGamePaused` true)
    (bind _returnvalue (`|CreateWidget` "/Game/BP/WBP/Play_WBP/Stack/WBP_Map_Stack.WBP_Map_Stack_C"))
    (`UserWidget.AddToViewport` _returnvalue 0)
    (`WidgetBlueprintLibrary.SetInputMode_UIOnlyEx` (`GameplayStatics.GetPlayerController` 0) _returnvalue)
    (`Widget.SetFocus` _returnvalue)))

(event `EnhancedInput|/Game/BP/ThirdPerson/ThirdPerson/Input/Actions/IA_UI_Charm`
  (params (ActionValue :type Boolean) (ElapsedSeconds :type "Float (double-precision)") (TriggeredSeconds :type "Float (double-precision)") (InputAction :type "InputAction Object Reference" :default "/Game/BP/ThirdPerson/ThirdPerson/Input/Actions/IA_UI_Charm.IA_UI_Charm"))
  ;[1 1 1] Map
  (:`Triggered`
    (`GameplayStatics.SetGamePaused` true)
    (bind _returnvalue (`|CreateWidget` "/Game/BP/WBP/Play_WBP/Stack/WBP_Charm_Stack.WBP_Charm_Stack_C"))
    (`UserWidget.AddToViewport` _returnvalue 0)
    (`WidgetBlueprintLibrary.SetInputMode_UIOnlyEx` (`GameplayStatics.GetPlayerController` 0) _returnvalue)
    (`Widget.SetFocus` _returnvalue)))

(event `self.ReceiveBeginPlay`
  ;[1 1 1] 코멘트
  (bind _asbp_mi_sin_jeon_game_mode_base (cast `/Game/BP/BP_MiSinJeonGameModeBase` (`GameplayStatics.GetGameMode`)))
  (set `self.GameMode` _asbp_mi_sin_jeon_game_mode_base)
  (bind _asseori (cast `Seori` (`GameplayStatics.GetPlayerPawn` 0)))
  (set `self.Seori` _asseori))

(fn `CallNextMonologue`
  (params (nextIndex :type Integer) (currWidget :type "Widget Object Reference"))
  (bind _gamemode (`self.GameMode`))
  (if (== nextIndex -1)
    (set `/Game/BP/BP_MiSinJeonGameModeBase.level` (+ (`/Game/BP/BP_MiSinJeonGameModeBase.level` _gamemode) 1) _gamemode)
    (set `/Game/BP/BP_MiSinJeonGameModeBase.index` 0 _gamemode)
    (`self.CloseDialogue` currWidget :!label _label)
    (`Seori.setTalking` (`self.Seori`) false)
    (bind _ashud_text (cast `/Game/BP/WBP/HUD_Text` currWidget))
    (set `/Game/BP/WBP/HUD_Text.isRemove` true _ashud_text)
    (else
      (set `/Game/BP/BP_MiSinJeonGameModeBase.index` nextIndex _gamemode)
      (bind _newparam (`/Game/BP/BP_MiSinJeonGameModeBase.FindCurrScript` _gamemode))
      (if (`KismetStringLibrary.EqualEqual_StrStr` (`.script_12_D19730314D570F5A73AD2FA074CCA8FA` (break `/Game/BP/BP_NPC/Script/BP_ScriptStruct` _newparam)))
        (goto _label)
        (else
          (bind _ashud_text_2 (cast `/Game/BP/WBP/HUD_Text` currWidget))
          (`/Game/BP/WBP/HUD_Text.setScript` _ashud_text_2 _newparam)))))
  (return))

(fn `CallNextScript`
  (params (currWidget :type "/Game/BP/WBP/HUD_Talking Object Reference") (index :type Integer))
  (bind _npc (`self.NPC`))
  (bind _npc_2 (`self.NPC`))
  (bind _gamemode (`self.GameMode`))
  (set `/Game/BP/BP_MiSinJeonGameModeBase.index` index (`self.GameMode`))
  (`/Engine/EditorBlueprintResources/StandardMacros.IsValid` _npc_2
    (:`Is Valid`
      (`NPC.Talk` _npc_2))
    (:`Is Not Valid`
      _))
  (bind _newparam (`/Game/BP/BP_MiSinJeonGameModeBase.FindCurrScript` (`self.GameMode`)))
  (bind (_script _isselectable _target _nextindex _endtalk) (break `/Game/BP/BP_NPC/Script/BP_ScriptStruct` _newparam))
  (if (`KismetStringLibrary.EqualEqual_StrStr` _script)
    (set `/Game/BP/BP_MiSinJeonGameModeBase.level` (+ (`/Game/BP/BP_MiSinJeonGameModeBase.level` _gamemode) 1) _gamemode)
    (set `/Game/BP/BP_MiSinJeonGameModeBase.index` 0 _gamemode)
    (elif _endtalk
      _
      (else
        (bind _output_get (set `self.currScript` _newparam))
        (`/Game/BP/WBP/HUD_Talking.setScript` currWidget _output_get)
        (if (`.isSelectable_15_769C9C8F4463251ACCE412A7411CFBBC` (break `/Game/BP/BP_NPC/Script/BP_ScriptStruct` _output_get))
          (bind _result (`/Game/BP/BP_MiSinJeonGameModeBase.FindCurrAnswer` (`self.GameMode`)))
          (bind _output_get_2 (set `self.currAnswer` _result))
          (`/Game/BP/WBP/HUD_Talking.setAnswer` currWidget _output_get_2))
        (return))))
  (`self.CloseDialogue` currWidget)
  (`/Engine/EditorBlueprintResources/StandardMacros.IsValid` _npc
    (:`Is Valid`
      (`NPC.setTalking` _npc false))
    (:`Is Not Valid`
      _))
  (`Seori.setTalking` (`self.Seori`) false)
  (return))

(fn `CheckAndWrapIndex`
  (params (currentIndex :type Integer) (ArrayLength :type Integer))
  (returns (WrappedIndex :type Boolean))
  (return (>= currentIndex ArrayLength)))

(fn `CloseDialogue`
  (params (currWidget :type "Widget Object Reference"))
  (`Widget.RemoveFromParent` currWidget)
  (bind _ashud_talking (cast `/Game/BP/WBP/HUD_Talking` currWidget))
  (set `/Game/BP/WBP/HUD_Talking.isRemove` true _ashud_talking)
  (`WidgetBlueprintLibrary.SetInputMode_GameOnly` self)
  (bind _asbp_seori (cast `/Game/BP/BP_Seori/BP_Seori` (`self.Seori`)))
  (set `/Game/BP/BP_Seori/BP_Seori.doneConversation` false _asbp_seori)
  (return))

(fn `OpenDialogue`
  (bind _currscript (`self.currScript`))
  (bind _gamemode (`self.GameMode`))
  (bind _returnvalue (`|CreateWidget` "/Game/BP/WBP/HUD_Talking.HUD_Talking_C"))
  (`WidgetBlueprintLibrary.SetInputMode_GameAndUIEx` self _returnvalue)
  (bind _newparam (`/Game/BP/BP_MiSinJeonGameModeBase.FindCurrScript` _gamemode))
  (if (`.isSelectable_15_769C9C8F4463251ACCE412A7411CFBBC` (break `/Game/BP/BP_NPC/Script/BP_ScriptStruct` _newparam))
    (bind _result (`/Game/BP/BP_MiSinJeonGameModeBase.FindCurrAnswer` _gamemode))
    (set `self.currAnswer` _result))
  (set `self.currScript` _newparam)
  (if (`KismetStringLibrary.EqualEqual_StrStr` (`.script_12_D19730314D570F5A73AD2FA074CCA8FA` (break `/Game/BP/BP_NPC/Script/BP_ScriptStruct` (`self.currScript`))))
    (bind _returnvalue_2 (`NPC.getName` (`self.NPC`)))
    (set `self.currScript` (make `/Game/BP/BP_NPC/Script/BP_ScriptStruct` "무슨일이야?" false _returnvalue_2)))
  (`/Game/BP/WBP/HUD_Talking.setScript` _returnvalue _currscript)
  (if (`.isSelectable_15_769C9C8F4463251ACCE412A7411CFBBC` (break `/Game/BP/BP_NPC/Script/BP_ScriptStruct` _currscript))
    (`/Game/BP/WBP/HUD_Talking.setAnswer` _returnvalue (`self.currAnswer`)))
  (`UserWidget.AddToViewport` _returnvalue 0)
  (return))

(fn `OpenMonologue`
  (params (chap :type Integer) (level :type Integer) (index :type Integer))
  (bind _gamemode (`self.GameMode`))
  (`/Game/BP/BP_MiSinJeonGameModeBase.setChap` _gamemode chap)
  (`/Game/BP/BP_MiSinJeonGameModeBase.setLevel` _gamemode level)
  (`/Game/BP/BP_MiSinJeonGameModeBase.setIndex` _gamemode index)
  (bind _returnvalue (`|CreateWidget` "/Game/BP/WBP/HUD_Text.HUD_Text_C"))
  (`WidgetBlueprintLibrary.SetInputMode_GameAndUIEx` self _returnvalue)
  (bind _newparam (`/Game/BP/BP_MiSinJeonGameModeBase.FindCurrScript` (`self.GameMode`)))
  (if (not (`KismetStringLibrary.EqualEqual_StrStr` (`.script_12_D19730314D570F5A73AD2FA074CCA8FA` (break `/Game/BP/BP_NPC/Script/BP_ScriptStruct` _newparam))))
    (`/Game/BP/WBP/HUD_Text.setScript` _returnvalue _newparam)
    (`UserWidget.AddToViewport` _returnvalue 0)))

(fn `setCurrAnswer`
  (params (answer :type "Array of /Game/BP/BP_NPC/Script/BP_AnswerStruct Structure"))
  (set `self.currAnswer` answer))

(fn `setCurrScript`
  (params (currScript :type "/Game/BP/BP_NPC/Script/BP_ScriptStruct Structure"))
  (set `self.currScript` currScript))

(fn `SetInputMode`
  (params (NowMode :type "/Game/BP/EInputMode Enum" :default "NewEnumerator0"))
  (bind _returnvalue (`GameplayStatics.GetPlayerController` 0))
  (bind _output_get (set `self.CurrentInputMode` NowMode))
  (if (`|EnumEquality` _output_get "NewEnumerator0")
    (`WidgetBlueprintLibrary.SetInputMode_GameOnly` _returnvalue)
    (else
      (`WidgetBlueprintLibrary.SetInputMode_UIOnlyEx` _returnvalue null))))

(fn `setNPC`
  (params (currNPC :type "NPC Object Reference"))
  (bind _output_get (set `self.NPC` currNPC))
  (`NPC.getName` _output_get))

(fn `setTarget`
  (params (target :type String))
  (set `self.target` target))

(fn `UserConstructionScript`)