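; BP_Turnstile is a ticket gate whose arm blocks the way until it is interacted with.
; When the arm is hit, it searches the Seori player's inventory, swaps ticket keys for the default key and sets the interacted state from a ticket check.
; Tick switches the arm's collision off while interacted.
; A player-tagged actor leaving the sphere clears the state, restoring the barrier.
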(event `self.ReceiveActorBeginOverlap`
  (params (OtherActor :type "Actor Object Reference")))

(event `self.ReceiveTick`
  (params (DeltaSeconds :type "Float (single-precision)"))
  (bind _arm (`self.arm`))
  (bind _returnvalue (`self.isInteracted`))
  (if _returnvalue
    (`PrimitiveComponent.SetCollisionEnabled` _arm "NoCollision")
    (else
      (`PrimitiveComponent.SetCollisionEnabled` _arm "QueryAndPhysics"))))

(event `self.sphereComponent.OnComponentEndOverlap`
  (params (OverlappedComponent :type "PrimitiveComponent Object Reference") (OtherActor :type "Actor Object Reference") (OtherComp :type "PrimitiveComponent Object Reference") (OtherBodyIndex :type Integer))
  (if (`self.ActorHasTag` OtherActor "Player")
    (`self.setInteracted` false)))

(event `self.arm.OnComponentHit`
  (params (HitComponent :type "PrimitiveComponent Object Reference") (OtherActor :type "Actor Object Reference") (OtherComp :type "PrimitiveComponent Object Reference") (NormalImpulse :type "Vector Structure") (Hit :type "HitResult Structure (by ref)"))
  (bind _ticketitemkey (`self.TicketItemKey`))
  (bind _asseori (cast `Seori` (`GameplayStatics.GetPlayerCharacter` 0)))
  (bind _returnvalue (`Seori.getInventory` _asseori))
  (bind _returnvalue_2 (`KismetArrayLibrary.Array_Contains` _returnvalue _ticketitemkey))
  (if _returnvalue_2
    (for (_array_element _array_index) _returnvalue
      (if (== _array_element _ticketitemkey)
        (`Seori.setInventoryItemKey` _asseori _array_index (`self.DEFALUT_ItemKey`))
        (`self.setInteracted` _returnvalue_2)))))

(fn `UserConstructionScript`)