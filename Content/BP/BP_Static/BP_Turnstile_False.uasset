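; Interactable turnstile that opens only when the Seori player character's open-turnstile value is true.
; OnInteract reads that value, disables collision on the Arm and calls TurnstileTurn to start the rotation.
; Tick turns the Arm by a fixed step per frame, stopping after a 120-degree turn.
; Arm collision is restored when an overlap with the sphere component ends.
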(event `self.ReceiveActorBeginOverlap`
  (params (OtherActor :type "Actor Object Reference")))

(event `self.ReceiveTick`
  (params (DeltaSeconds :type "Float (single-precision)"))
  (if (`self.doRotation`)
    (`SceneComponent.K2_AddLocalRotation` (`self.arm`) (struct :`Yaw` 2.0) false false)
    (bind _output_get (set `self.RotateVector` (+ (`self.RotateVector`) 2.0)))
    (if (>= _output_get 120.0)
      (set `self.doRotation` false)
      (set `self.RotateVector` 0.0))))

(event `self.sphereComponent.OnComponentEndOverlap`
  (params (OverlappedComponent :type "PrimitiveComponent Object Reference") (OtherActor :type "Actor Object Reference") (OtherComp :type "PrimitiveComponent Object Reference") (OtherBodyIndex :type Integer))
  (`PrimitiveComponent.SetCollisionEnabled` (`self.arm`) "QueryAndPhysics"))

(event `self.OnInteract`
  (bind _asseori (cast `Seori` (`GameplayStatics.GetPlayerCharacter` 0)))
  (bind _returnvalue (`Seori.getOpenTurnstile` _asseori))
  (if _returnvalue
    (`PrimitiveComponent.SetCollisionEnabled` (`self.arm`) "NoCollision")
    (`self.TurnstileTurn`)))

(fn `TurnstileTurn`
  (set `self.doRotation` true))

(fn `UserConstructionScript`)