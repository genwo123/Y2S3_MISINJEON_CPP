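; Interactable table prop that triggers the chapter-opening charm sequence on first use and opens the charm stack UI afterward.
; Before chapter 1, interacting plays the charm video for its duration, opens dialogue, then teleports the player to the "Come2F" start behind a loading widget, resetting time and advancing the game mode to chapter 1.
; A sphere overlap toggles the guide's visibility for the player.
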(event `self.ReceiveBeginPlay`
  (bind _asbp_mi_sin_jeon_game_mode_base (cast `/Game/BP/BP_MiSinJeonGameModeBase` (`GameplayStatics.GetGameMode`)))
  (set `self.GameModeBase` _asbp_mi_sin_jeon_game_mode_base)
  (bind _asbp_misinjeon_player_controller (cast `/Game/BP/BP_MisinjeonPlayerController` (`GameplayStatics.GetPlayerController` 0)))
  (set `self.PlayerController` _asbp_misinjeon_player_controller))

(event `self.OnInteract`
  (bind _returnvalue (`GameplayStatics.GetGameMode`))
  (bind _returnvalue_2 (`GameplayStatics.GetPlayerController` 0))
  (bind _returnvalue_3 (`GameplayStatics.GetPlayerPawn` 0))
  (bind _gamemodebase (`self.GameModeBase`))
  (bind _mediaplayer (`self.MediaPlayer`))
  (bind _asbp_mi_sin_jeon_game_mode_base (cast `/Game/BP/BP_MiSinJeonGameModeBase` (`GameplayStatics.GetGameMode`)))
  (if (< (`/Game/BP/BP_MiSinJeonGameModeBase.chap` _asbp_mi_sin_jeon_game_mode_base) 1)
    (`self.DisableInput` (`self.PlayerController`))
    (`MediaPlayer.OpenSource` _mediaplayer "/Game/UIUX/UMG/U_Media/charm_video.charm_video")
    (bind _returnvalue_4 (`|CreateWidget` "/Game/BP/WBP/IntroWBP/WBP_Cinematic.WBP_Cinematic_C"))
    (`UserWidget.AddToViewport` _returnvalue_4 0)
    (`KismetSystemLibrary.Delay` 0.2)
    (bind _output_get (set `self.timespan` (`MediaPlayer.GetDuration` _mediaplayer)))
    (`KismetSystemLibrary.Delay` (`KismetMathLibrary.GetTotalSeconds` _output_get))
    (`Widget.RemoveFromParent` _returnvalue_4)
    (`/Game/BP/BP_MiSinJeonGameModeBase.setChap` _gamemodebase 0)
    (`/Game/BP/BP_MiSinJeonGameModeBase.setLevel` _gamemodebase 9)
    (`/Game/BP/BP_MiSinJeonGameModeBase.setIndex` _gamemodebase 1)
    (bind _openedwidget (`/Game/BP/BP_MisinjeonPlayerController.OpenDialogue` (`self.PlayerController`)))
    (`KismetSystemLibrary.Delay` 4.0)
    (bind _returnvalue_5 (`|CreateWidget` "/Game/BP/WBP/Play_WBP/WBP_Loding.WBP_Loding_C"))
    (`UserWidget.AddToViewport` _returnvalue_5 1)
    (`WidgetBlueprintLibrary.SetInputMode_UIOnlyEx` _returnvalue_2 _returnvalue_5)
    (`self.K2_SetActorTransform` _returnvalue_3 (`self.GetTransform` (`GameModeBase.K2_FindPlayerStart` _returnvalue _returnvalue_2 "Come2F")) false true)
    (`self.K2_SetActorRelativeRotation` _returnvalue_3 (struct :`Yaw` 90.0) false false)
    (bind _aswb_misingeon_instance (cast `/Game/BP/Saveing/WB_MisingeonInstance` (`GameplayStatics.GetGameInstance`)))
    (set `/Game/BP/Saveing/WB_MisingeonInstance.time` 0 _aswb_misingeon_instance)
    (bind _asbp_mi_sin_jeon_game_mode_base_2 (cast `/Game/BP/BP_MiSinJeonGameModeBase` _returnvalue))
    (`/Game/BP/BP_MiSinJeonGameModeBase.setChap` _asbp_mi_sin_jeon_game_mode_base_2 1)
    (`/Game/BP/BP_MiSinJeonGameModeBase.setLevel` _asbp_mi_sin_jeon_game_mode_base_2 0)
    (`/Game/BP/BP_MiSinJeonGameModeBase.setIndex` _asbp_mi_sin_jeon_game_mode_base_2 0)
    (`KismetSystemLibrary.Delay` 2.0)
    (`/Game/BP/BP_MisinjeonPlayerController.CloseDialogue` (`self.PlayerController`) _openedwidget)
    (`Widget.RemoveFromParent` _returnvalue_5)
    (`WidgetBlueprintLibrary.SetInputMode_GameOnly` _returnvalue_2)
    (`self.setInteracted` false)
    (`KismetSystemLibrary.Delay` 0.2)
    (else
      (bind _returnvalue_6 (`|CreateWidget` "/Game/BP/WBP/Play_WBP/Stack/WBP_Charm_Stack.WBP_Charm_Stack_C"))
      (`UserWidget.AddToViewport` _returnvalue_6 0)
      (`WidgetBlueprintLibrary.SetInputMode_UIOnlyEx` (`GameplayStatics.GetPlayerController` 0) _returnvalue_6)
      (`Widget.SetFocus` _returnvalue_6)
      (`self.setInteracted` false)
      (`KismetSystemLibrary.Delay` 0.2))))

(event `self.sphereComponent.OnComponentEndOverlap`
  (params (OverlappedComponent :type "PrimitiveComponent Object Reference") (OtherActor :type "Actor Object Reference") (OtherComp :type "PrimitiveComponent Object Reference") (OtherBodyIndex :type Integer))
  (if (`self.ActorHasTag` OtherActor "Player")
    (`SceneComponent.SetVisibility` (`self.Guide`) false false)))

(event `self.sphereComponent.OnComponentBeginOverlap`
  (params (OverlappedComponent :type "PrimitiveComponent Object Reference") (OtherActor :type "Actor Object Reference") (OtherComp :type "PrimitiveComponent Object Reference") (OtherBodyIndex :type Integer) (bFromSweep :type Boolean) (SweepResult :type "HitResult Structure (by ref)"))
  (if (`self.ActorHasTag` OtherActor "Player")
    (`SceneComponent.SetVisibility` (`self.Guide`) true false)))

(fn `UserConstructionScript`)