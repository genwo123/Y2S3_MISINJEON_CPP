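; BP_LeesoeOutDoor is an interactable door that offers a level move to Fortune_Interior with the "ComeOut" spawn tag.
; A sphere component shows or hides a Guide prompt as the player-tagged actor enters or leaves.
; Interacting opens WBP_MoveLevel_Choice with UI-only input and writes hard-coded chapter, level and index values to the game mode.
; After a short delay it refocuses the widget and clears the interacted flag.
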(event `self.OnInteract`
  (bind _returnvalue (`|CreateWidget` "/Game/BP/WBP/Play_WBP/Choice/WBP_MoveLevel_Choice.WBP_MoveLevel_Choice_C"))
  (set `/Game/BP/WBP/Play_WBP/Choice/WBP_MoveLevel_Choice.spawnTag` "ComeOut" _returnvalue)
  (set `/Game/BP/WBP/Play_WBP/Choice/WBP_MoveLevel_Choice.ToLevelName` "Fortune_Interior" _returnvalue)
  (`UserWidget.AddToViewport` _returnvalue 0)
  (`WidgetBlueprintLibrary.SetInputMode_UIOnlyEx` (`GameplayStatics.GetPlayerController` 0) _returnvalue)
  (bind _asbp_mi_sin_jeon_game_mode_base (cast `/Game/BP/BP_MiSinJeonGameModeBase` (`GameplayStatics.GetGameMode`)))
  (`/Game/BP/BP_MiSinJeonGameModeBase.setChap` _asbp_mi_sin_jeon_game_mode_base 9)
  (`/Game/BP/BP_MiSinJeonGameModeBase.setLevel` _asbp_mi_sin_jeon_game_mode_base 0)
  (`/Game/BP/BP_MiSinJeonGameModeBase.setIndex` _asbp_mi_sin_jeon_game_mode_base 5)
  (`KismetSystemLibrary.Delay` 0.2)
  (`Widget.SetFocus` _returnvalue)
  (`self.setInteracted` false))

(event `self.sphereComponent.OnComponentEndOverlap`
  (params (OverlappedComponent :type "PrimitiveComponent Object Reference") (OtherActor :type "Actor Object Reference") (OtherComp :type "PrimitiveComponent Object Reference") (OtherBodyIndex :type Integer))
  (if (`self.ActorHasTag` OtherActor "Player")
    (`SceneComponent.SetVisibility` (`self.Guide`) false false)))

(event `self.sphereComponent.OnComponentBeginOverlap`
  (params (OverlappedComponent :type "PrimitiveComponent Object Reference") (OtherActor :type "Actor Object Reference") (OtherComp :type "PrimitiveComponent Object Reference") (OtherBodyIndex :type Integer) (bFromSweep :type Boolean) (SweepResult :type "HitResult Structure (by ref)"))
  (if (`self.ActorHasTag` OtherActor "Player")
    (`SceneComponent.SetVisibility` (`self.Guide`) true false)))

(fn `UserConstructionScript`)