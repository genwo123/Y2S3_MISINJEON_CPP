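; Base goblin enemy Blueprint that detects the Seori player and performs a melee attack on her.
; Pawn sensing sets a "HasSeenPlayer?" blackboard flag on the AI controller when it sees Seori.
; AttackPlayer sphere-traces just ahead for Seori, then after a short delay plays the attack montage and immediately deals damage, with no re-check of range.
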(event `self.PawnSensing.OnSeePawn`
  (params (Pawn :type "Pawn Object Reference"))
  (cast `Seori` Pawn)
  (`BlackboardComponent.SetValueAsBool` (`AIBlueprintHelperLibrary.GetBlackboard` (`AIBlueprintHelperLibrary.GetAIController` self)) "HasSeenPlayer?" true))

(event `Attack Player`
  (bind _returnvalue (`self.K2_GetActorLocation`))
  (bind (_outhit _returnvalue_2) (`KismetSystemLibrary.SphereTraceSingleForObjects` _returnvalue (+ _returnvalue (* (`KismetMathLibrary.GetForwardVector` (`self.K2_GetActorRotation`)) 100.0)) 100.0 (`|MakeArray` "ObjectTypeQuery3" :!type "EObjectTypeQuery Enum")))
  (if _returnvalue_2
    (bind _asseori (cast `Seori` (`.HitActor` (`GameplayStatics.BreakHitResult` _outhit))))
    (`KismetSystemLibrary.Delay` 1.0)
    (`self.PlayAnimMontage` "/Game/BP/AI/Animation/ANI_Mon_Goblin_01_B_Attack_00_Montage.ANI_Mon_Goblin_01_B_Attack_00_Montage")
    (`Seori.TakeDamage` _asseori 1)))

(fn `UserConstructionScript`)