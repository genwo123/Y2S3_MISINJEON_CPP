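; Pojangmacha (street food stall) NPC that opens a fixed dialogue when the player talks to it.
; A sphere trigger shows the Guide component when the player enters, then hides it, clears the talking state and resets rotation on exit.
; On talking, it registers with the player controller, sets the GameMode's chapter, level and index, opens dialogue, calls Listen and hides the guide.
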(event `self.ReceiveBeginPlay`
  (set `self.thisNPC` self)
  (bind _asbp_misinjeon_player_controller (cast `/Game/BP/BP_MisinjeonPlayerController` (`GameplayStatics.GetPlayerController` 0)))
  (set `self.PlayerController` _asbp_misinjeon_player_controller))

(event `self.onTalking`
  (bind _thisnpc (`self.thisNPC`))
  (bind _playercontroller (`self.PlayerController`))
  (`/Engine/EditorBlueprintResources/StandardMacros.IsValid` _thisnpc
    (:`Is Valid`
      (bind _returnvalue (`self.isTalking` _thisnpc))
      (if _returnvalue
        (`/Game/BP/BP_MisinjeonPlayerController.setNPC` _playercontroller self)
        (bind _asbp_mi_sin_jeon_game_mode_base (cast `/Game/BP/BP_MiSinJeonGameModeBase` (`GameplayStatics.GetGameMode`)))
        (`/Game/BP/BP_MiSinJeonGameModeBase.setChap` _asbp_mi_sin_jeon_game_mode_base 9)
        (`/Game/BP/BP_MiSinJeonGameModeBase.setLevel` _asbp_mi_sin_jeon_game_mode_base 0)
        (`/Game/BP/BP_MiSinJeonGameModeBase.setIndex` _asbp_mi_sin_jeon_game_mode_base 3)
        (`/Game/BP/BP_MisinjeonPlayerController.OpenDialogue` _playercontroller)
        (`self.Listen` _thisnpc)
        (`SceneComponent.SetVisibility` (`self.Guide`) false false)))))

(event `self.sphereComponent.OnComponentEndOverlap`
  (params (OverlappedComponent :type "PrimitiveComponent Object Reference") (OtherActor :type "Actor Object Reference") (OtherComp :type "PrimitiveComponent Object Reference") (OtherBodyIndex :type Integer))
  (bind _thisnpc (`self.thisNPC`))
  (if (`self.ActorHasTag` OtherActor "Player")
    (`/Engine/EditorBlueprintResources/StandardMacros.IsValid` _thisnpc
      (:`Is Valid`
        (`self.setTalking` _thisnpc false)
        (`self.ResetRotation` _thisnpc)
        (`SceneComponent.SetVisibility` (`self.Guide`) false false)))))

(event `self.sphereComponent.OnComponentBeginOverlap`
  (params (OverlappedComponent :type "PrimitiveComponent Object Reference") (OtherActor :type "Actor Object Reference") (OtherComp :type "PrimitiveComponent Object Reference") (OtherBodyIndex :type Integer) (bFromSweep :type Boolean) (SweepResult :type "HitResult Structure (by ref)"))
  (if (`self.ActorHasTag` OtherActor "Player")
    (`SceneComponent.SetVisibility` (`self.Guide`) true false)))

(fn `UserConstructionScript`)