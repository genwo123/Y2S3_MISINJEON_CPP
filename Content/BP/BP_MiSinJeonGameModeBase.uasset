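; Game mode that tracks story progress as Chap, Level and Index and looks up the current script and answer choices.
; BeginPlay loads the three values from WB_MisingeonInstance, and each setter writes its value back to that game instance.
; FindCurrScript and FindCurrAnswer concatenate them into row names for DT_ScriptTable and DT_AnswerTable.
; A missing script row returns a non-selectable "None" default, while answers collect up to two rows.
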(event `self.ReceiveBeginPlay`
  (bind _aswb_misingeon_instance (cast `/Game/BP/Saveing/WB_MisingeonInstance` (`GameplayStatics.GetGameInstance`)))
  (set `self.chap` (`/Game/BP/Saveing/WB_MisingeonInstance.chap` _aswb_misingeon_instance))
  (set `self.level` (`/Game/BP/Saveing/WB_MisingeonInstance.level` _aswb_misingeon_instance))
  (set `self.index` (`/Game/BP/Saveing/WB_MisingeonInstance.index` _aswb_misingeon_instance)))

(fn `FindCurrAnswer`
  (returns (result :type "Array of /Game/BP/BP_NPC/Script/BP_AnswerStruct Structure"))
  (bind _curranswer (`self.currAnswer`))
  (`KismetArrayLibrary.Array_Clear` (`self.currAnswer`))
  (for _index (range 1 3)
    (bind _returnvalue (`|GetDataTableRow` "/Game/BP/BP_NPC/Script/DT_AnswerTable.DT_AnswerTable" (`KismetStringLibrary.Conv_StringToName` (`KismetStringLibrary.Concat_StrStr` (`KismetStringLibrary.Conv_IntToString` (`self.chap`)) (`KismetStringLibrary.Conv_IntToString` (`self.level`)) (`KismetStringLibrary.Conv_IntToString` (`self.index`)) (`KismetStringLibrary.Conv_IntToString` _index))))
      (:`then`
        (`KismetArrayLibrary.Array_Add` _curranswer _returnvalue))))
  (return _curranswer))

(fn `FindCurrScript`
  (returns (NewParam :type "/Game/BP/BP_NPC/Script/BP_ScriptStruct Structure"))
  (bind _returnvalue (`KismetStringLibrary.Conv_IntToString` (`self.chap`)))
  (bind _returnvalue_2 (`KismetStringLibrary.Conv_IntToString` (`self.level`)))
  (bind _returnvalue_3 (`KismetStringLibrary.Conv_IntToString` (`self.index`)))
  (`KismetSystemLibrary.PrintString` (`KismetStringLibrary.Concat_StrStr` _returnvalue "," _returnvalue_2 "," _returnvalue_3))
  (bind _returnvalue_4 (`|GetDataTableRow` "/Game/BP/BP_NPC/Script/DT_ScriptTable.DT_ScriptTable" (`KismetStringLibrary.Conv_StringToName` (`KismetStringLibrary.Concat_StrStr` _returnvalue _returnvalue_2 _returnvalue_3)))
    (:`then`
      (bind _output_get (set `self.currScriptStruct` _returnvalue_4))
      (return _output_get))
    (:`RowNotFound`
      (return (make `/Game/BP/BP_NPC/Script/BP_ScriptStruct` "None")))))

(fn `setChap`
  (params (chap :type Integer))
  (bind _output_get (set `self.chap` chap))
  (bind _aswb_misingeon_instance (cast `/Game/BP/Saveing/WB_MisingeonInstance` (`GameplayStatics.GetGameInstance`)))
  (set `/Game/BP/Saveing/WB_MisingeonInstance.chap` _output_get _aswb_misingeon_instance))

(fn `setIndex`
  (params (index :type Integer))
  (bind _output_get (set `self.index` index))
  (bind _aswb_misingeon_instance (cast `/Game/BP/Saveing/WB_MisingeonInstance` (`GameplayStatics.GetGameInstance`)))
  (set `/Game/BP/Saveing/WB_MisingeonInstance.index` _output_get _aswb_misingeon_instance))

(fn `setLevel`
  (params (level :type Integer))
  (bind _output_get (set `self.level` level))
  (bind _aswb_misingeon_instance (cast `/Game/BP/Saveing/WB_MisingeonInstance` (`GameplayStatics.GetGameInstance`)))
  (set `/Game/BP/Saveing/WB_MisingeonInstance.level` _output_get _aswb_misingeon_instance))

(fn `UserConstructionScript`)